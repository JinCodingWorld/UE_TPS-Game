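; BP_TPSPlayer is a third-person shooter player Blueprint whose events, including BeginPlay, Tick and the IA_Sniper input, are all empty.
; An unconnected node chain holds hitscan sniper-style fire, so it never runs.
; When the handgun is not in use, that chain traces the Visibility channel along the camera's forward vector and spawns an explosion emitter at the hit location.
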(event `self.ReceiveTick`
  (params (DeltaSeconds :type "Float (single-precision)")))

(event `self.ReceiveBeginPlay`)

(event `EnhancedInput|/Game/Input/IA_Sniper`
  (params (ActionValue :type Boolean) (ElapsedSeconds :type "Float (double-precision)") (TriggeredSeconds :type "Float (double-precision)") (InputAction :type "InputAction Object Reference" :default "/Game/Input/IA_Sniper.IA_Sniper")))

(fn `UserConstructionScript`)